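; Base Blueprint for destructible environment objects that take damage and are destroyed when their health runs out.
; Any damage is passed as a negative change to the TDSHealth component; point and radial damage events are empty.
; Each health change spawns a BP_DisplayDamageActor at a randomly jittered offset, initialized with current health and damage.
; On death, the actor is destroyed with a collapse sound and explosion particle at its location.
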(event OnHealthChange(TDSHealth)
  (params (Health :type Float%20%28single-precision%29) (Damage :type Float%20%28single-precision%29))
  (bind _returnvalue (Game|SpawnActorfromClass "/Game/Blueprint/InteractionEnvironmet/DisplayDamage/BP_DisplayDamageActor.BP_DisplayDamageActor_C" (Math|Transform|MakeTransform (+ (Transformation|GetActorLocation) (+ (Variables|Default|GetLocalPointSpawnHealthNumber) (Math|Vector|MakeVector (Math|Random|RandomFloatinRange -2e+01 2e+01) (Math|Random|RandomFloatinRange -2e+01 2e+01) 0.0)))) "Undefined" "MultiplyWithRoot" 0 0))
  (Default|InitActor _returnvalue Health Damage))

(event OnDead(TDSHealth)
  (CallFunction|DestroyActor))

(event EventBeginPlay)

(event Game|Damage|EventAnyDamage
  (params (Damage :type Float%20%28single-precision%29) (DamageType :type Damage%20Type%20Object%20Reference) (InstigatedBy :type Controller%20Object%20Reference) (DamageCauser :type Actor%20Object%20Reference))
  (Class|TDSHealthComponent|ChangeHealthValue (Variables|Default|GetTDSHealth) (* Damage -1.0)))

(event Game|Damage|EventPointDamage
  (params (Damage :type Float%20%28single-precision%29) (DamageType :type Damage%20Type%20Object%20Reference) (HitLocation :type Vector :default "0, 0, 0") (HitNormal :type Vector :default "0, 0, 0") (HitComponent :type Primitive%20Component%20Object%20Reference) (BoneName :type Name :default "None") (ShotFromDirection :type Vector :default "0, 0, 0") (InstigatedBy :type Controller%20Object%20Reference) (DamageCauser :type Actor%20Object%20Reference) (HitInfo :type Hit%20Result%20Structure%20%28by%20ref%29)))

(event Game|Damage|EventRadialDamage
  (params (DamageReceived :type Float%20%28single-precision%29) (DamageType :type Damage%20Type%20Object%20Reference) (Origin :type Vector :default "0, 0, 0") (HitInfo :type Hit%20Result%20Structure%20%28by%20ref%29) (InstigatedBy :type Controller%20Object%20Reference) (DamageCauser :type Actor%20Object%20Reference)))

(fn ConstructionScript)

(fn DestroyActor
  (bind _returnvalue (Transformation|GetActorLocation))
  (Actor|DestroyActor)
  (Audio|SpawnSoundatLocation "/Game/StarterContent/Audio/Collapse01.Collapse01" _returnvalue "0, 0, 0" 1.0 1.0 0.0 0 0)
  (Effects|SpawnEmitteratLocation "/Game/StarterContent/Particles/P_Explosion.P_Explosion" _returnvalue))