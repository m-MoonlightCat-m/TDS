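; Base enemy character for a networked top-down shooter, handling AI attacks, hit reactions, death and loot drops.
; Passes ranged flag and attack distance to the AI blackboard; light and heavy attacks play multicast montages whose notifies trigger server-side sphere traces or spell projectiles.
; Health changes show damage numbers and randomly trigger confusion, hit animations or slowdowns.
; Death unpossesses, drops a randomly assigned ammo item if present, then ragdolls after the montage.
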(event OnHealthChange(TDSHealth)
  (params (Health :type Float%20%28single-precision%29) (Damage :type Float%20%28single-precision%29))
  (bind _returnvalue (Game|SpawnActorfromClass "/Game/TDS/Blueprint/InteractionEnvironmet/DisplayDamage/BP_DisplayDamage.BP_DisplayDamage_C" (Math|Transform|MakeTransform (+ (Transformation|GetActorLocation) (+ (Variables|Default|GetSpawnOffsetLocalDamage) (Math|Vector|MakeVector (Math|Random|RandomFloatinRange -2e+01 2e+01) (Math|Random|RandomFloatinRange -2e+01 2e+01) 0.0)))) "Undefined" "MultiplyWithRoot" 0 0))
  (Default|InitActor _returnvalue Health Damage)
  (Networking|SwitchHasAuthority
    (:Authority
      (if (> (Math|Random|RandomFloat) (Variables|Chance|GetConfusionChance))
        (CallFunction|ConfusionEnableTimer)
        (else
          (CallFunction|HitAnim)))
      (if (> (Math|Random|RandomFloat) (Variables|Chance|GetSlowDawnSpeedChance))
        (Variables|Flag|SetSlowDawnSpeed true)
        (Utilities|Time|SetTimerbyEvent (delegate Custom|SlowDawnDisable) 2.0)))))

(event OnDead(TDSHealth)
  (Networking|SwitchHasAuthority
    (:Authority
      (CallFunction|DeadEventMulticast))))

(event Custom|SlowDawnDisable
  (Variables|Flag|SetSlowDawnSpeed false))

(event Custom|LongRangAttackLight_Multicast
  (params (SelectedLightAttack :type Anim%20Montage%20Object%20Reference))
  (bind _arrow1 (Variables|Default|GetArrow1))
  ;[1 1 1] Melle\Long Rang Attack
  (Networking|SwitchHasAuthority
    (:Authority
      (bind _notifyname (Animation|Montage|PlayMontage (Variables|Character|GetMesh) SelectedLightAttack)
        (:OnCompleted
          (CallFunction|SetStateAttack true :!label _label))
        (:OnInterrupted
          (goto _label))
        (:OnNotifyBegin
          (if (== _notifyname "Attack")
            (bind _returnvalue (Game|SpawnActorfromClass "/Game/TDS/Blueprint/EnemyCharacter/Spell/BP_Spell_Light.BP_Spell_Light_C" (Math|Transform|MakeTransform (+ (Math|Vector|GetForwardVector _arrow1) (Transformation|GetWorldLocation _arrow1)) (Transformation|GetWorldRotation _arrow1)) "AlwaysSpawn" "MultiplyWithRoot" self 0))
            (Class|ProjectileDefault|InitProjectile _returnvalue (Utilities|Struct|MakeProjectileInfo "/Game/TDS/Blueprint/EnemyCharacter/Spell/BP_Spell_Light.BP_Spell_Light_C" "/Game/TDS/Items/EnemyItem/MagicSphereBullet.MagicSphereBullet" "0.000000,0.000000,0.000000|0.000000,0.000000,-0.000000|1.000000,1.000000,1.000000" "/Game/TDS/Effect/VFX/Magic_Downpour_VFX/VFX/Magic_Downpour_VFX/NS_Magic_Downpour_Wizard_Staff_LightSpell.NS_Magic_Downpour_Wizard_Staff_LightSpell" "0.000000,0.000000,0.000000|0.000000,0.000000,-0.000000|1.000000,1.000000,1.000000" 2e+01 2e+01 2e+03 3e+03 "SurfaceType_Default" 0 "SurfaceType_Default"))))))
    (:Remote
      (Animation|PlayAnimMontage SelectedLightAttack 1.0 "None"))))

(event Custom|MeleeAttackLight_Multicast
  (params (SelectedLigthAttack :type Anim%20Montage%20Object%20Reference))
  (bind _baselightdamage (Variables|Combat|GetBaseLightDamage))
  ;[1 1 1] Melle\Long Rang Attack
  (Networking|SwitchHasAuthority
    (:Authority
      (bind _notifyname (Animation|Montage|PlayMontage (Variables|Character|GetMesh) SelectedLigthAttack)
        (:OnCompleted
          (CallFunction|SetStateAttack true :!label _label))
        (:OnInterrupted
          (goto _label))
        (:OnNotifyBegin
          (if (== _notifyname "Attack") ; Light
            (Utilities|MeleeTrace (Variables|Combat|GetStartLightTraceDistance) (Variables|Combat|GetEndLightTraceDistance) (Variables|Combat|GetLightRadius) (Math|Random|RandomFloatinRange (- _baselightdamage 1e+01) (+ _baselightdamage 2e+01)))))))
    (:Remote
      (Animation|PlayAnimMontage SelectedLigthAttack 1.0 "None"))))

(event Custom|MeleeAttackHeavy_Multicast
  (params (SelectedHeavyAttack :type Anim%20Montage%20Object%20Reference))
  (bind _baseheavydamage (Variables|Combat|GetBaseHeavyDamage))
  ;[1 1 1] Melle\Long Rang Attack
  (Networking|SwitchHasAuthority
    (:Authority
      (bind _notifyname (Animation|Montage|PlayMontage (Variables|Character|GetMesh) SelectedHeavyAttack)
        (:OnCompleted
          (CallFunction|SetStateMovement true :!label _label)
          (CallFunction|SetStateAttack true))
        (:OnInterrupted
          (goto _label))
        (:OnNotifyBegin
          (if (== _notifyname "Attack") ; Heavy
            (Utilities|MeleeTrace (Variables|Combat|GetStartHeavyTraceDistance) (Variables|Combat|GetEndHeavyTraceDistance) (Variables|Combat|GetHeavyRadius) (Math|Random|RandomFloatinRange (- _baseheavydamage 1e+01) (+ _baseheavydamage 5e+01)))))))
    (:Remote
      (Animation|PlayAnimMontage SelectedHeavyAttack 1.0 "None"))))

(event Custom|LongRangeAttackHeavy_Multicast
  (params (SelectedLongRangeHeavyAttack :type Anim%20Montage%20Object%20Reference))
  (bind _arrow1 (Variables|Default|GetArrow1))
  ;[1 1 1] Melle\Long Rang Attack
  (Networking|SwitchHasAuthority
    (:Authority
      (bind _notifyname (Animation|Montage|PlayMontage (Variables|Character|GetMesh) SelectedLongRangeHeavyAttack)
        (:OnCompleted
          (CallFunction|SetStateAttack true :!label _label))
        (:OnInterrupted
          (goto _label))
        (:OnNotifyBegin
          (if (== _notifyname "Attack")
            (bind _returnvalue (Game|SpawnActorfromClass "/Game/TDS/Blueprint/EnemyCharacter/Spell/BP_Spell_Heavy.BP_Spell_Heavy_C" (Math|Transform|MakeTransform (+ (Math|Vector|GetForwardVector _arrow1) (Transformation|GetWorldLocation _arrow1)) (Transformation|GetWorldRotation _arrow1)) "AlwaysSpawn" "MultiplyWithRoot" self 0))
            (Class|ProjectileDefault|InitProjectile _returnvalue (Utilities|Struct|MakeProjectileInfo "/Game/TDS/Blueprint/EnemyCharacter/Spell/BP_Spell_Heavy.BP_Spell_Heavy_C" "/Game/TDS/Items/EnemyItem/MagicSphereBullet.MagicSphereBullet" "0.000000,0.000000,0.000000|0.000000,0.000000,-0.000000|1.000000,1.000000,1.000000" "/Game/TDS/Effect/VFX/Magic_Downpour_VFX/VFX/Magic_Downpour_VFX/NS_Magic_Downpour_Wizard_Staff_HeavySpell.NS_Magic_Downpour_Wizard_Staff_HeavySpell" "0.000000,0.000000,0.000000|0.000000,0.000000,-0.000000|1.000000,1.000000,1.000000" 6e+01 3e+01 2e+03 4e+03 "SurfaceType_Default" 0 "SurfaceType_Default" 0 0 0 2e+02 2e+02 6e+01))))))
    (:Remote
      (Animation|PlayAnimMontage SelectedLongRangeHeavyAttack 1.0 "None"))))

(event Custom|DeadEvent_Multicast
  (bind _deadanimmontage (Variables|Animation|GetDeadAnimMontage))
  (Networking|SwitchHasAuthority
    (:Authority
      (Animation|Montage|PlayMontage (Variables|Character|GetMesh) _deadanimmontage
        (:then
          (Components|Movement|StopMovementImmediately (Variables|Character|GetCharacterMovement))
          (CallFunction|DeadEvent))
        (:OnCompleted
          (CallFunction|EnableRagdoll))))
    (:Remote
      (Animation|PlayAnimMontage _deadanimmontage 1.0 "None"))))

(event Custom|PlayAnim_Multicast
  (params (AnimMontage :type Anim%20Montage%20Object%20Reference) (InPlayRate :type Float%20%28single-precision%29) (StartSectionName :type Name))
  (Animation|PlayAnimMontage AnimMontage InPlayRate StartSectionName))

(event Custom|EnableRagdoll
  (bind _mesh (Variables|Character|GetMesh))
  (Collision|SetCollisionEnabled _mesh "PhysicsOnly")
  (Collision|SetCollisionProfileName _mesh "PhysicsActor" true :!class /Script/Engine.PrimitiveComponent)
  (Collision|SetCollisionResponsetoChannel (Variables|Default|GetCapsuleComponent) "ECC_Pawn" "ECR_Ignore")
  (Collision|SetCollisionObjectType _mesh "ECC_PhysicsBody")
  (Physics|SetSimulatePhysics _mesh true))

(event EventBeginPlay
  (CallFunction|InitDropComponent)
  (bind _asbp_aicontroller (Utilities|Casting|CastToBP_AIController (AI|GetAIController (Components|GetOwner))))
  (AI|Components|Blackboard|SetValueasBool (Variables|/Script/AIModule.AIController|GetBlackboard _asbp_aicontroller) (Utilities|Name|MakeLiteralName "IsRangedEnemy") (Variables|Combat|GetbIsRangedAttack))
  (AI|Components|Blackboard|SetValueasFloat (Variables|/Script/AIModule.AIController|GetBlackboard _asbp_aicontroller) (Utilities|Name|MakeLiteralName "AttackDistance") (Variables|Combat|GetAttackDistanceChar)))

(event EventTick
  (params (DeltaSeconds :type Float%20%28single-precision%29))
  (Variables|Default|SetDeltaTime DeltaSeconds)
  (Utilities|ChangeSpeedbyHit))

(event EventMeleeAttackHeavy
  (bind _heavyattackanim (Variables|Combat|GetHeavyAttackAnim))
  ;[1 1 1] Melle\Long Rang Attack
  (CallFunction|SetStateAttack false)
  (CallFunction|SetStateMovement false)
  (bind _output_get (Variables|Anim|SetSelectedHeavyAttack (Utilities|Array|Get(acopy) _heavyattackanim (Math|Random|RandomInteger (Utilities|Array|Length _heavyattackanim)))))
  (CallFunction|MeleeAttackHeavyMulticast _output_get))

(event Game|Damage|EventAnyDamage
  (params (Damage :type Float%20%28single-precision%29) (DamageType :type Damage%20Type%20Object%20Reference) (InstigatedBy :type Controller%20Object%20Reference) (DamageCauser :type Actor%20Object%20Reference))
  (Class|TDSHealthComponent|ChangeHealthValueonServer (Variables|Default|GetTDSHealth) (* Damage -1.0))
  (Variables|Default|SetLastInstigated InstigatedBy))

(event EventMeleeAttackLight
  (bind _lightattackanim (Variables|Combat|GetLightAttackAnim))
  ;[1 1 1] Melle\Long Rang Attack
  (CallFunction|SetStateAttack false)
  (bind _output_get (Variables|Anim|SetSelectedLigthAttack (Utilities|Array|Get(acopy) _lightattackanim (Math|Random|RandomInteger (Utilities|Array|Length _lightattackanim)))))
  (CallFunction|MeleeAttackLightMulticast _output_get))

(event EventLongRangeAttackHeavy
  (bind _heavyattackanim (Variables|Combat|GetHeavyAttackAnim))
  ;[1 1 1] Melle\Long Rang Attack
  (CallFunction|SetStateAttack false)
  (bind _output_get (Variables|Anim|SetSelectedLongRangeHeavyAttack (Utilities|Array|Get(acopy) _heavyattackanim (Math|Random|RandomInteger (Utilities|Array|Length _heavyattackanim)))))
  (CallFunction|LongRangeAttackHeavyMulticast _output_get))

(event EventLongRangeAttackLight
  (bind _lightattackanim (Variables|Combat|GetLightAttackAnim))
  ;[1 1 1] Melle\Long Rang Attack
  (CallFunction|SetStateAttack false)
  (bind _output_get (Variables|Anim|SetSelectedLongRangeLightAttack (Utilities|Array|Get(acopy) _lightattackanim (Math|Random|RandomInteger (Utilities|Array|Length _lightattackanim)))))
  (CallFunction|LongRangAttackLightMulticast _output_get))

(fn ConstructionScript)

(fn SetStateMovement
  (params (CanMove :type Boolean))
  (Variables|Combat|SetCanMovePawn CanMove))

(fn SetStateAttack
  (params (CanAttack :type Boolean))
  (Variables|Combat|SetCamAttackPawn CanAttack))

(fn DeadEvent
  (bind _dropcomponent (Variables|Default|GetDropComponent))
  (Pawn|UnPossess (Pawn|GetController))
  (Actor|SetLifeSpan 2e+01)
  (CallFunction|SetStateMovement false)
  (CallFunction|SetStateAttack false)
  (Utilities|IsValid _dropcomponent
    (:Is%20Valid
      (Default|Drop _dropcomponent))))

(fn InitDropComponent
  (bind _returnvalue (Math|Random|RandomIntegerinRange 0 3))
  (bind _returnvalue_2 (Utilities|Select :Index _returnvalue :Option%200 "RifleMKType" :Option%201 "ShotGunType" :Option%202 "SniperRifle" :Option%203 "GrenadeLauncher"))
  (Networking|SwitchHasAuthority
    (:Authority
      (if (> (Math|Random|RandomFloat) (Variables|Chance|GetDropChance))
        (bind _returnvalue_3 (AddComponent|AddBPDropItemComponent))
        (Variables|Default|SetDropComponent _returnvalue_3)
        (Variables|/Game/TDS/Blueprint/BP_DropItemComponent.BP_DropItemComponent_C|SetType _returnvalue_3 _returnvalue_2)
        (Utilities|FlowControl|Sequence
          (:then_0
            (switch Utilities|FlowControl|Switch|SwitchonEWeaponType _returnvalue_2
              (:RifleMKType
                (LocalVariables|SetCout 30))
              (:ShotGunType
                (LocalVariables|SetCout 12))
              (:SniperRifle
                (LocalVariables|SetCout 6))
              (:GrenadeLauncher
                (LocalVariables|SetCout 2))))
          (:then_1
            (Variables|/Game/TDS/Blueprint/BP_DropItemComponent.BP_DropItemComponent_C|SetCout _returnvalue_3 (LocalVariables|GetCout))))))))

(fn ConfusionEnableTimer
  (bind _confusionanim (Variables|Animation|GetConfusionAnim))
  (CallFunction|SetStateMovement false)
  (bind _output_get (Variables|Animation|SetCurrentMontage (Utilities|Array|Get(acopy) _confusionanim (Math|Random|RandomIntegerinRange 0 (- (Utilities|Array|Length _confusionanim) 1)))))
  (Utilities|Time|SetTimerbyFunctionName 0 "ConfusionDisabledTimer" (Animation|GetPlayLength _output_get))
  (CallFunction|PlayAnimMulticast (Variables|Animation|GetCurrentMontage) 1.0 "None")
  (Variables|/Script/Engine.CharacterMovementComponent|SetMaxWalkSpeed (Variables|Character|GetCharacterMovement) 0.0)
  (Variables|Flag|SetbIsConfused true))

(fn ConfusionDisabledTimer
  (CallFunction|SetStateMovement true)
  (Variables|/Script/Engine.CharacterMovementComponent|SetMaxWalkSpeed (Variables|Character|GetCharacterMovement) (Variables|Combat|GetMax%20Walk%20Speed))
  (Variables|Flag|SetbIsConfused false))

(fn HitAnim
  (if (not (Variables|Flag|GetbIsConfused))
    (if (> (Math|Random|RandomFloat) (Variables|Chance|GetHitAnimChance))
      (CallFunction|PlayAnimMulticast (Variables|Animation|GetConfusedAnimMontage) 1.0 "None"))))

(fn CanAttack
  (return (Variables|Combat|GetCamAttackPawn)))

(fn CanMove
  (return (Variables|Combat|GetCanMovePawn)))