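; Base AI character for the wolf boss's minions, with health, light and heavy melee attacks and death handling.
; Attacks multicast random montages, with server-side notifies running sphere traces that damage players.
; Hits spawn damage numbers and randomly trigger confusion stuns, flinches or a timed slowdown applied on Tick.
; Death notifies the boss found in the level, plays a montage, unpossesses the pawn and ragdolls it on the server.
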(event OnHealthChange(TDSHealth)
  (params (Health :type Float%20%28single-precision%29) (Damage :type Float%20%28single-precision%29))
  (bind _returnvalue (Game|SpawnActorfromClass "/Game/TDS/Blueprint/InteractionEnvironmet/DisplayDamage/BP_DisplayDamage.BP_DisplayDamage_C" (Math|Transform|MakeTransform (+ (Transformation|GetActorLocation) (+ (Variables|Default|GetSpawnOffsetLocalDamage) (Math|Vector|MakeVector (Math|Random|RandomFloatinRange -2e+01 2e+01) (Math|Random|RandomFloatinRange -2e+01 2e+01) 0.0)))) "Undefined" "MultiplyWithRoot" 0 0))
  (Default|InitActor _returnvalue Health Damage)
  (Networking|SwitchHasAuthority
    (:Authority
      (if (> (Math|Random|RandomFloat) (Variables|Chance|GetConfusionChance))
        (CallFunction|ConfusionEnableTimer)
        (else
          (CallFunction|HitAnim)))
      (if (> (Math|Random|RandomFloat) (Variables|Chance|GetSlowDawnSpeedChance))
        (Variables|Default|SetSlowDawnSpeed true)
        (Utilities|Time|SetTimerbyEvent (delegate Custom|SlowDawnDisable) 2.0)))))

(event OnDead(TDSHealth)
  (Networking|SwitchHasAuthority
    (:Authority
      (bind _returnvalue (Actor|GetActorOfClass "/Game/TDS/Blueprint/EnemyCharacter/Boss/BP_CharacterEnemy_Boss.BP_CharacterEnemy_Boss_C"))
      (Default|WolfDead _returnvalue)
      (Variables|Default|SetbIsDead true)
      (CallFunction|DeadEventMulticast))))

(event Custom|SlowDawnDisable
  (Variables|Default|SetSlowDawnSpeed false))

(event Custom|DeadEvent_Multicast
  (bind _deadanimmontage (Variables|Animation|GetDeadAnimMontage))
  (Networking|SwitchHasAuthority
    (:Authority
      (Animation|Montage|PlayMontage (Variables|Character|GetMesh) _deadanimmontage
        (:then
          (Components|Movement|StopMovementImmediately (Variables|Character|GetCharacterMovement))
          (CallFunction|DeadEvent))
        (:OnCompleted
          (CallFunction|EnableRagdoll))))
    (:Remote
      (Animation|PlayAnimMontage _deadanimmontage 1.0 "None"))))

(event Custom|EnableRagdoll
  (bind _mesh (Variables|Character|GetMesh))
  (bind _capsulecomponent (Variables|Collision|GetCapsuleComponent))
  (Collision|SetCollisionEnabled _mesh "PhysicsOnly")
  (Collision|SetCollisionProfileName _mesh "PhysicsActor" true :!class /Script/Engine.PrimitiveComponent)
  (Collision|SetCollisionResponsetoChannel _capsulecomponent "ECC_Pawn" "ECR_Ignore")
  (Collision|SetCollisionObjectType _mesh "ECC_WorldStatic")
  (Collision|SetCollisionResponsetoChannel _capsulecomponent "ECC_GameTraceChannel6" "ECR_Ignore")
  (Physics|SetSimulatePhysics _mesh true))

(event Custom|MeleeAttackLight_Multicast
  (params (SelectedLightAttack :type Anim%20Montage%20Object%20Reference))
  (bind _baselightdamage (Variables|Combat|GetBaseLightDamage))
  (Networking|SwitchHasAuthority
    (:Authority
      (bind _notifyname (Animation|Montage|PlayMontage (Variables|Character|GetMesh) SelectedLightAttack)
        (:OnCompleted
          (CallFunction|SetStateAttack true :!label _label))
        (:OnInterrupted
          (goto _label))
        (:OnNotifyBegin
          (if (== _notifyname "Attack") ; Light
            (Utilities|MeleeTrace (Variables|Combat|GetStartLightTraceDistance) (Variables|Combat|GetEndLightTraceDistance) (Variables|Combat|GetLightRadius) (Math|Random|RandomFloatinRange (- _baselightdamage 1e+01) (+ _baselightdamage 2e+01)))))))
    (:Remote
      (Animation|PlayAnimMontage SelectedLightAttack 1.0 "None"))))

(event Custom|MeleeAttackHeavy_Multicast
  (params (SelectedHeavyAttack :type Anim%20Montage%20Object%20Reference))
  (bind _baseheavydamage (Variables|Combat|GetBaseHeavyDamage))
  (Networking|SwitchHasAuthority
    (:Authority
      (bind _notifyname (Animation|Montage|PlayMontage (Variables|Character|GetMesh) SelectedHeavyAttack)
        (:OnCompleted
          (CallFunction|SetStateMovement true :!label _label)
          (CallFunction|SetStateAttack true))
        (:OnInterrupted
          (goto _label))
        (:OnNotifyBegin
          (if (== _notifyname "Attack") ; Heavy
            (Utilities|MeleeTrace (Variables|Combat|GetStartHeavyTraceDistance) (Variables|Combat|GetEndHeavyTraceDistance) (Variables|Combat|GetHeavyRadius) (Math|Random|RandomFloatinRange (- _baseheavydamage 1e+01) (+ _baseheavydamage 5e+01)))))))
    (:Remote
      (Animation|PlayAnimMontage SelectedHeavyAttack 1.0 "None"))))

(event EventBeginPlay
  (bind _asbp_aicontroller (Utilities|Casting|CastToBP_AIController (AI|GetAIController (Components|GetOwner))))
  (AI|Components|Blackboard|SetValueasFloat (Variables|/Script/AIModule.AIController|GetBlackboard _asbp_aicontroller) (Utilities|Name|MakeLiteralName "AttackDistance") (Variables|Combat|GetAttackDistanceChar)))

(event EventTick
  (params (DeltaSeconds :type Float%20%28single-precision%29))
  (Variables|Default|SetDeltaTime DeltaSeconds)
  (Utilities|ChangeSpeedbyHit))

(event EventMeleeAttackHeavy
  (bind _heavyattackanim (Variables|Combat|GetHeavyAttackAnim))
  (CallFunction|SetStateAttack false)
  (CallFunction|SetStateMovement false)
  (bind _output_get (Variables|Default|SetSelectedHeavyAttack (Utilities|Array|Get(acopy) _heavyattackanim (Math|Random|RandomInteger (Utilities|Array|Length _heavyattackanim)))))
  (CallFunction|MeleeAttackHeavyMulticast _output_get))

(event Game|Damage|EventAnyDamage
  (params (Damage :type Float%20%28single-precision%29) (DamageType :type Damage%20Type%20Object%20Reference) (InstigatedBy :type Controller%20Object%20Reference) (DamageCauser :type Actor%20Object%20Reference))
  (Class|TDSHealthComponent|ChangeHealthValueonServer (Variables|Default|GetTDSHealth) (* Damage -1.0)))

(event EventMeleeAttackLight
  (bind _lightattackanim (Variables|Combat|GetLightAttackAnim))
  (CallFunction|SetStateAttack false)
  (bind _output_get (Variables|Default|SetSelectedLightAttack (Utilities|Array|Get(acopy) _lightattackanim (Math|Random|RandomInteger (Utilities|Array|Length _lightattackanim)))))
  (CallFunction|MeleeAttackLightMulticast _output_get))

(fn ConstructionScript)

(fn SetStateMovement
  (params (CanMove :type Boolean))
  (Variables|Combat|SetCanMovePawn CanMove))

(fn SetStateAttack
  (params (CanAttack :type Boolean))
  (Variables|Combat|SetCamAttackPawn CanAttack))

(fn DeadEvent
  (Pawn|UnPossess (Pawn|GetController))
  (Actor|SetLifeSpan 2e+01)
  (CallFunction|SetStateMovement false)
  (CallFunction|SetStateAttack false))

(fn ConfusionEnableTimer
  (bind _confusionanim (Variables|Animation|GetConfusionAnim))
  (CallFunction|SetStateMovement false)
  (bind _output_get (Variables|Animation|SetCurrentMontage (Utilities|Array|Get(acopy) _confusionanim (Math|Random|RandomIntegerinRange 0 (- (Utilities|Array|Length _confusionanim) 1)))))
  (Utilities|Time|SetTimerbyFunctionName 0 "ConfusionDisabledTimer" (Animation|GetPlayLength _output_get))
  (Animation|PlayAnimMontage (Variables|Animation|GetCurrentMontage) 1.0 "None")
  (Variables|/Script/Engine.CharacterMovementComponent|SetMaxWalkSpeed (Variables|Character|GetCharacterMovement) 0.0)
  (Variables|Default|SetbIsConfused true))

(fn ConfusionDisabledTimer
  (CallFunction|SetStateMovement true)
  (Variables|/Script/Engine.CharacterMovementComponent|SetMaxWalkSpeed (Variables|Character|GetCharacterMovement) (Variables|Default|GetMax%20Walk%20Speed))
  (Variables|Default|SetbIsConfused false))

(fn HitAnim
  (if (not (Variables|Default|GetbIsConfused))
    (if (> (Math|Random|RandomFloat) (Variables|Chance|GetHitAnimChance))
      (Animation|PlayAnimMontage (Variables|Animation|GetConfusedAnimMontage) 1.0 "None"))))

(fn CanAttack
  (return (Variables|Combat|GetCamAttackPawn)))

(fn CanMove
  (return (Variables|Combat|GetCanMovePawn)))