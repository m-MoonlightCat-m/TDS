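; Boss turret actor that periodically launches magic-orb missiles for its owning boss character.
; On BeginPlay it loops two gyroscope mesh animations, and the server starts a repeating timer.
; While the boss has health, each tick of the timer plays the Shoot timeline, whose event spawns and initializes a BP_MissleTurret projectile along the arrow component.
; Once the boss's health is depleted, the next timer call clears the timer.
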(event Custom|FireRocketEvent
  (bind _returnvalue (Components|GetOwner))
  (bind _projectileinfo (Utilities|Struct|MakeProjectileInfo "/Game/TDS/Blueprint/EnemyCharacter/Boss/Turret/BP_MissleTurret.BP_MissleTurret_C" "/Game/TDS/Items/EnemyItem/MagicSphereBullet.MagicSphereBullet" "0.000000,0.000000,0.000000|0.000000,0.000000,-0.000000|1.000000,1.000000,1.000000" "/Game/TDS/Effect/VFX/Magic_Downpour_VFX/VFX/Magic_Downpour_VFX/NS_Magic_Downpour_Wizard_Staff_Infinite.NS_Magic_Downpour_Wizard_Staff_Infinite" "0.000000,0.000000,0.000000|0.000000,0.000000,-0.000000|1.000000,1.000000,1.000000" 1.0 2e+01 5e+02 1e+03 "SurfaceType_Default" 0 "SurfaceType_Default" 0 "/Game/TDS/Effect/VFX/Magic_Downpour_VFX/VFX/Magic_Downpour_VFX/NS_Magic_Downpour_Wizard_Staff_End.NS_Magic_Downpour_Wizard_Staff_End" "/Game/TDS/Blueprint/Sounds/Audio/Effect/MagicBalle.MagicBalle" 1.5e+02 5e+01 3e+01 2.0))
  (bind _arrow (Variables|Default|GetArrow))
  (bind _asbp_character_enemy_boss (Utilities|Casting|CastToBP_CharacterEnemy_Boss _returnvalue))
  (bind _returnvalue_2 (Class|TDSHealthComponent|GetCurrentHealth (Variables|/Game/TDS/Blueprint/EnemyCharacter/BP_CharacterEnemy_Base.BP_CharacterEnemy_Base_C|GetTDSHealth _asbp_character_enemy_boss)))
  (if (> _returnvalue_2 0.0)
    (Timeline|Shoot Play
      (:Shoot
        (bind _returnvalue_3 (Game|SpawnActorfromClass "/Game/TDS/Blueprint/EnemyCharacter/Boss/Turret/BP_MissleTurret.BP_MissleTurret_C" (Math|Transform|MakeTransform (+ (Math|Vector|GetForwardVector _arrow) (Transformation|GetWorldLocation _arrow)) (Transformation|GetWorldRotation _arrow)) "AlwaysSpawn" "MultiplyWithRoot" _returnvalue (.ProjectileInitSpeed (Utilities|Struct|BreakProjectileInfo _projectileinfo)) 0))
        (Class|ProjectileDefault|InitProjectile _returnvalue_3 _projectileinfo)))
    (else
      (Utilities|Time|ClearandInvalidateTimerbyHandle (Variables|Default|GetFireRocket_HandleTimer)))))

(event EventBeginPlay
  (Components|Animation|PlayAnimation (Variables|Default|GetSkeletalMesh1) "/Game/TDS/Items/EnemyItem/magic-gyroscope/source/Gyroscope_Torus001_Anim.Gyroscope_Torus001_Anim" true)
  (Components|Animation|PlayAnimation (Variables|Default|GetSkeletalMesh) "/Game/TDS/Items/EnemyItem/magic-gyroscope/source/Gyroscope_Sphere001_Anim.Gyroscope_Sphere001_Anim" true)
  (Networking|SwitchHasAuthority
    (:Authority
      (if (Networking|IsServer)
        (bind _returnvalue (Utilities|Time|SetTimerbyEvent (delegate Custom|FireRocketEvent) 3.0 true))
        (Variables|Default|SetFireRocket_HandleTimer _returnvalue)))))

(event Collision|EventActorBeginOverlap
  (params (OtherActor :type Actor%20Object%20Reference)))

(event EventTick
  (params (DeltaSeconds :type Float%20%28single-precision%29)))

(fn ConstructionScript
  (|CallParentFunction))