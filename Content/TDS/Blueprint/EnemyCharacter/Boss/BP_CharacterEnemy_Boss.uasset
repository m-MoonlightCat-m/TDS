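; Boss enemy character that carries an attached turret and adds minion spawning, self-healing and a temporary shield.
; Looping timers spawn minions up to a cap, killing survivors once the boss dies, and occasionally trigger a montage-driven heal that pauses movement and attacks.
; Health changes at or below half raise a damage-immune shield, with timers handling its duration and cooldown.
; Tick prints health and minion count for debugging.
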(event OnHealthChange(TDSHealth)
  (params (Health :type Float%20%28single-precision%29) (Damage :type Float%20%28single-precision%29))
  (if (> Health 0.0)
    (if (not (Variables|Default|GetbIsHealing))
      (if (Variables|Default|GetbCanUpSheild)
        (bind _returnvalue (Class|TDSHealthComponent|GetMaxHealth (Variables|Default|GetTDSHealth)))
        (if (>= (* _returnvalue 0.5) Health)
          (CallFunction|SheildUp))))
    (else
      (Utilities|Time|ClearandInvalidateTimerbyHandle (Variables|Default|GetShieldUpTimerHandle))
      (Utilities|Time|ClearandInvalidateTimerbyHandle (Variables|Default|GetShieldDownTimerHandle)))))

(event Custom|WolfSpawnEvent
  (CallFunction|WolfSpawn))

(event Custom|Healing
  (bind _tdshealth (Variables|Default|GetTDSHealth))
  (bind _niagara (Variables|Default|GetNiagara))
  (bind _tdshealth_2 (Variables|Default|GetTDSHealth))
  (bind _returnvalue (Class|TDSHealthComponent|GetCurrentHealth _tdshealth))
  (if (> _returnvalue 0.0)
    (if (not (Variables|Default|GetbIsSheild))
      (bind _returnvalue_2 (Class|TDSHealthComponent|GetMaxHealth _tdshealth))
      (if (< _returnvalue _returnvalue_2)
        (if (< (Math|Random|RandomFloat) 0.6)
          (CallFunction|SetStateMovement false)
          (CallFunction|SetStateAttack false)
          (Variables|Default|SetbIsHealing true)
          (Animation|Montage|PlayMontage (Variables|Character|GetMesh) (Variables|Default|GetHealingAnim)
            (:OnCompleted
              (Utilities|IsValid _niagara
                (:Is%20Valid
                  (Class|NiagaraComponent|SetAsset _niagara "/Game/TDS/Effect/VFX/Vefects/Zap_VFX/VFX/Zap/Particles/NS_Zap_01_Red.NS_Zap_01_Red" true)
                  (bind _returnvalue_3 (Class|TDSHealthComponent|GetCurrentHealth _tdshealth_2))
                  (bind _returnvalue_4 (Class|TDSHealthComponent|GetMaxHealth _tdshealth_2))
                  (if (> (+ _returnvalue_3 (Variables|Default|GetHealingValue)) _returnvalue_4)
                    (Class|TDSHealthComponent|SetCurrentHealth _tdshealth_2 _returnvalue_4)
                    (else
                      (Class|TDSHealthComponent|SetCurrentHealth _tdshealth_2 (+ _returnvalue_3 (Variables|Default|GetHealingValue)))))
                  (CallFunction|SetStateMovement true)
                  (CallFunction|SetStateAttack true)
                  (Variables|Default|SetbIsHealing false))
                (:Is%20Not%20Valid
                  (Components|DestroyComponent _niagara))))))))
    (else
      (Utilities|Time|ClearandInvalidateTimerbyHandle (Variables|Default|GetHealingTimerHandle)))))

(event EventBeginPlay
  (bind _mesh (Variables|Character|GetMesh))
  (|CallParentFunction)
  (bind _returnvalue (Game|SpawnActorfromClass "/Game/TDS/Blueprint/EnemyCharacter/Boss/Turret/BP_TurretBoss.BP_TurretBoss_C" (Math|Conversions|ToTransform(Vector) (Transformation|GetSocketLocation _mesh "TurretSocket")) "AlwaysSpawn" "MultiplyWithRoot" self 0))
  (Transformation|AttachComponentToComponent (Variables|/Script/Engine.Actor|GetRootComponent _returnvalue) _mesh "TurretSocket" "SnapToTarget" "SnapToTarget" "SnapToTarget" true)
  (bind _returnvalue_2 (Utilities|Time|SetTimerbyEvent (delegate Custom|WolfSpawnEvent) 3.0 true))
  (Variables|Default|SetWolfSpawn_HandleTimer _returnvalue_2)
  (bind _returnvalue_3 (Utilities|Time|SetTimerbyEvent (delegate Custom|Healing) 2e+01 true))
  (Variables|Default|SetHealingTimerHandle _returnvalue_3))

(event EventTick
  (params (DeltaSeconds :type Float%20%28single-precision%29))
  (|CallParentFunction DeltaSeconds)
  (bind _returnvalue (Class|TDSHealthComponent|GetCurrentHealth (Variables|Default|GetTDSHealth)))
  (Development|PrintString (Utilities|String|ToString(Float) _returnvalue) true true "(R=0.000000,G=0.660000,B=1.000000,A=1.000000)" 0.0)
  (Development|PrintString (Utilities|String|ToString(Integer) (Variables|Default|GetWolf)) true true "(R=1.000000,G=0.556703,B=0.093750,A=1.000000)" 0.0))

(fn ConstructionScript
  (|CallParentFunction))

(fn WolfDead
  (Variables|Default|SetWolf (- (Variables|Default|GetWolf) 1)))

(fn WolfSpawn
  (bind _returnvalue (Class|TDSHealthComponent|GetCurrentHealth (Variables|Default|GetTDSHealth)))
  (if (> _returnvalue 0.0)
    (if (< (Variables|Default|GetWolf) (Variables|Default|GetMaxWolf))
      (Game|SpawnActorfromClass "/Game/TDS/Blueprint/EnemyCharacter/Boss/Wolf/BP_Minion_Base.BP_Minion_Base_C" (Math|Transform|MakeTransform (+ (Transformation|GetActorLocation) "150.000000,150.000000,0.000000") (Transformation|GetActorRotation)) "AlwaysSpawn" "MultiplyWithRoot" 0 false 0)
      (Variables|Default|SetWolf (+ (Variables|Default|GetWolf) 1)))
    (else
      (Utilities|Time|ClearandInvalidateTimerbyHandle (Variables|Default|GetWolfSpawn_HandleTimer))
      (bind _outactors (Actor|GetAllActorsOfClass "/Game/TDS/Blueprint/EnemyCharacter/Boss/Wolf/BP_Minion_Base.BP_Minion_Base_C"))
      (for _array_element _outactors
        (if (not (Variables|/Game/TDS/Blueprint/EnemyCharacter/Boss/Wolf/BP_Minion_Base.BP_Minion_Base_C|GetbIsDead _array_element))
          (Game|Damage|ApplyDamage _array_element 5e+03 0 0))))))

(fn SheildUp
  (Variables|Default|SetbIsSheild true)
  (Variables|Default|SetbCanUpSheild false)
  (CallFunction|SetStateMovement false)
  (Animation|PlayAnimMontage "/Game/TDS/Character/Enemy/Boss/Animation/AM_BossShield.AM_BossShield" 1.0 "None")
  (CallFunction|SetStateMovement true)
  (Class|NiagaraComponent|SetAsset (Variables|Default|GetNiagaraShield) "/Game/TDS/Effect/VFX/sA_PickupSet_1/Fx/NiagaraSystems/NS_Shield_3.NS_Shield_3" true)
  (Variables|/Script/TDS.TDSHealthComponent|SetbIsImmunToDamage (Variables|Default|GetTDSHealth) true)
  (bind _returnvalue (Utilities|Time|SetTimerbyFunctionName 0 "SheildDown" 1e+01))
  (Variables|Default|SetShieldUpTimerHandle _returnvalue))

(fn SheildDown
  (Class|NiagaraComponent|SetAsset (Variables|Default|GetNiagaraShield) 0 true)
  (Variables|/Script/TDS.TDSHealthComponent|SetbIsImmunToDamage (Variables|Default|GetTDSHealth) false)
  (Variables|Default|SetbIsSheild false)
  (bind _returnvalue (Utilities|Time|SetTimerbyFunctionName 0 "CanUseShield" 2e+01))
  (Variables|Default|SetShieldDownTimerHandle _returnvalue))

(fn CanUseShield
  (Variables|Default|SetbCanUpSheild true))