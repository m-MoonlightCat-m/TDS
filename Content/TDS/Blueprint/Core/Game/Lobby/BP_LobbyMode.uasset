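; Lobby game mode that seats joining players, manages their color and hat choices, and server-travels to the selected level.
; PostLogin spawns a lobby character at a free TargetPoint, tracked in an occupancy map, with a random available color.
; Cosmetic changes go through BP_LobbyState's blocked lists, and logout releases the point, color and hat.
; It pushes level changes to controllers and can save cosmetics by player name in the GameInstance.
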(event Custom|LaunchGame
  (Development|ExecuteConsoleCommand (Utilities|String|Append "servertravel " (Utilities|String|ToString(Name) (Variables|Default|GetSelectedLevel))) (Game|GetPlayerController 0)))

(event Custom|SaveColorForPlayers
  (bind _asbp_game_instance (Utilities|Casting|CastToBP_GameInstance (Game|GetGameInstance)))
  (for _array_element (Variables|Default|GetPlayerController)
    (bind _asbp_lobby_player_controller (Utilities|Casting|CastToBP_LobbyPlayerController _array_element))
    (Utilities|Map|Add (Variables|/Game/TDS/Blueprint/Core/Game/BP_GameInstance.BP_GameInstance_C|GetColorForPlayers _asbp_game_instance) (PlayerState|GetPlayerName (Variables|/Script/Engine.Controller|GetPlayerState _asbp_lobby_player_controller)) (Variables|/Game/TDS/Blueprint/Core/Game/Lobby/BP_LobbyCharacter.BP_LobbyCharacter_C|GetTrueColor (Variables|/Game/TDS/Blueprint/Core/Game/Lobby/BP_LobbyPlayerController.BP_LobbyPlayerController_C|GetLobbyCharacter _asbp_lobby_player_controller)))
    (Utilities|Map|Add (Variables|/Game/TDS/Blueprint/Core/Game/BP_GameInstance.BP_GameInstance_C|GetHatMeshForPlayers _asbp_game_instance) (PlayerState|GetPlayerName (Variables|/Script/Engine.Controller|GetPlayerState _asbp_lobby_player_controller)) (Variables|/Game/TDS/Blueprint/Core/Game/Lobby/BP_LobbyCharacter.BP_LobbyCharacter_C|GetTrueHatMesh (Variables|/Game/TDS/Blueprint/Core/Game/Lobby/BP_LobbyPlayerController.BP_LobbyPlayerController_C|GetLobbyCharacter _asbp_lobby_player_controller)))
    (Default|RemoveAllWidget _asbp_lobby_player_controller)))

(event Custom|UpdateLevelName
  (params (SelectedLevel :type Name))
  (Variables|Default|SetSelectedLevel SelectedLevel)
  (for _array_element (Variables|Default|GetPlayerController)
    (bind _asbp_lobby_player_controller (Utilities|Casting|CastToBP_LobbyPlayerController _array_element))
    (Default|UpdateLobbyWidgetonClient _asbp_lobby_player_controller (Variables|Default|GetSelectedLevel))))

(event Custom|UpdateHatForCharacter
  (params (Mesh :type Static%20Mesh%20Object%20Reference) (Controller :type BP%20Lobby%20Player%20Controller%20Object%20Reference))
  (bind _asbp_lobby_state (Utilities|Casting|CastToBP_LobbyState (Game|GetGameState)))
  (Default|SelectedNewHatonServer _asbp_lobby_state (Variables|/Game/TDS/Blueprint/Core/Game/Lobby/BP_LobbyCharacter.BP_LobbyCharacter_C|GetTrueHatMesh (Variables|/Game/TDS/Blueprint/Core/Game/Lobby/BP_LobbyPlayerController.BP_LobbyPlayerController_C|GetLobbyCharacter Controller)) Mesh)
  (Default|UpdateLobbycharacterHateMeshParam Controller Mesh))

(event Custom|UpdateColorForCharacter
  (params (Color :type Material%20Interface%20Object%20Reference) (Controller :type BP%20Lobby%20Player%20Controller%20Object%20Reference))
  (bind _asbp_lobby_state (Utilities|Casting|CastToBP_LobbyState (Game|GetGameState)))
  (Default|SelectedNewColoronServer _asbp_lobby_state (Variables|/Game/TDS/Blueprint/Core/Game/Lobby/BP_LobbyCharacter.BP_LobbyCharacter_C|GetTrueColor (Variables|/Game/TDS/Blueprint/Core/Game/Lobby/BP_LobbyPlayerController.BP_LobbyPlayerController_C|GetLobbyCharacter Controller)) Color)
  (Default|UpdateLobbyCharacterColorParam Controller Color))

(event EventBeginPlay)

(event EventTick
  (params (DeltaSeconds :type Float%20%28single-precision%29)))

(event EventPostLogin
  (params (NewPlayer :type Player%20Controller%20Object%20Reference))
  (bind _targetpoint (Variables|Default|GetTargetPoint))
  (bind _targetpoint_2 (Variables|Default|GetTargetPoint))
  (bind _keys (Utilities|Map|Keys _targetpoint))
  (if (> (Utilities|Array|Length _keys) 0)
    _
    (else
      (bind _outactors (Actor|GetAllActorsOfClass "/Script/Engine.TargetPoint"))
      (for _array_element _outactors
        (Utilities|Map|Add _targetpoint _array_element false))))
  (bind _asbp_lobby_player_controller (Utilities|Casting|CastToBP_LobbyPlayerController NewPlayer))
  (Utilities|Array|Add (Variables|Default|GetPlayerController) _asbp_lobby_player_controller)
  (Variables|/Game/TDS/Blueprint/Core/Game/Lobby/BP_LobbyPlayerController.BP_LobbyPlayerController_C|SetCurrentLevelByServer _asbp_lobby_player_controller (Variables|Default|GetSelectedLevel))
  (bind _keys_2 (Utilities|Map|Keys _targetpoint_2))
  (bind _array_element_2 (Utilities|Array|ForEachLoopwithBreak _keys_2 :!label _label)
    (:LoopBody
      (if (not (.Value (Utilities|Map|Find _targetpoint_2 _array_element_2)))
        (Utilities|Map|Add _targetpoint_2 _array_element_2 true)
        (bind _returnvalue (Game|SpawnActorfromClass "/Game/TDS/Blueprint/Core/Game/Lobby/BP_LobbyCharacter.BP_LobbyCharacter_C" (Transformation|GetActorTransform _array_element_2) "AlwaysSpawn" "MultiplyWithRoot" 0 0))
        (Variables|/Game/TDS/Blueprint/Core/Game/Lobby/BP_LobbyPlayerController.BP_LobbyPlayerController_C|SetOccupidPoint _asbp_lobby_player_controller _array_element_2)
        (Default|SaveLobbyCharacter _asbp_lobby_player_controller _returnvalue)
        (CallFunction|SetRandomColorforCharacter _asbp_lobby_player_controller)
        (goto _label Break)))))

(event EventOnLogout
  (params (ExitingController :type Controller%20Object%20Reference))
  (bind _asbp_lobby_player_controller (Utilities|Casting|CastToBP_LobbyPlayerController ExitingController))
  (Utilities|Array|RemoveItem (Variables|Default|GetPlayerController) _asbp_lobby_player_controller)
  (Utilities|Map|Add (Variables|Default|GetTargetPoint) (Variables|/Game/TDS/Blueprint/Core/Game/Lobby/BP_LobbyPlayerController.BP_LobbyPlayerController_C|GetOccupidPoint _asbp_lobby_player_controller) false)
  (bind _asbp_lobby_state (Utilities|Casting|CastToBP_LobbyState (Game|GetGameState)))
  (Default|AddorRemoveColortoBlock _asbp_lobby_state (Variables|/Game/TDS/Blueprint/Core/Game/Lobby/BP_LobbyCharacter.BP_LobbyCharacter_C|GetTrueColor (Variables|/Game/TDS/Blueprint/Core/Game/Lobby/BP_LobbyPlayerController.BP_LobbyPlayerController_C|GetLobbyCharacter _asbp_lobby_player_controller)) true)
  (Default|AddorRemoveHattoBlock _asbp_lobby_state (Variables|/Game/TDS/Blueprint/Core/Game/Lobby/BP_LobbyCharacter.BP_LobbyCharacter_C|GetTrueHatMesh (Variables|/Game/TDS/Blueprint/Core/Game/Lobby/BP_LobbyPlayerController.BP_LobbyPlayerController_C|GetLobbyCharacter _asbp_lobby_player_controller)) true))

(fn ConstructionScript)

(fn SetRandomColorforCharacter
  (params (Controller :type BP%20Lobby%20Player%20Controller%20Object%20Reference))
  (bind _asbp_lobby_state (Utilities|Casting|CastToBP_LobbyState (Game|GetGameState)))
  (bind _aviablecolorout (Default|GetAviableColor _asbp_lobby_state))
  (LocalVariables|SetNewColor (Utilities|Array|Get(acopy) _aviablecolorout (Math|Random|RandomInteger (- (Utilities|Array|Length _aviablecolorout) 1))))
  (Default|AddorRemoveColortoBlock _asbp_lobby_state (LocalVariables|GetNewColor) false)
  (Default|UpdateLobbyCharacterColorParam Controller (LocalVariables|GetNewColor)))