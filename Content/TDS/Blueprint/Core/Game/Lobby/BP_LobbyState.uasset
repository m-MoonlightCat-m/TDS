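; Lobby state Blueprint that tracks which player colors and hat meshes are taken in the lobby.
; Server-side events swap, add or remove entries in the blocked color and hat lists.
; After each change, it loops over the BP_LobbyMode player controllers and pushes the updated list to their lobby widgets through client update calls.
; Getters expose both blocked lists and compute the colors still available from the full color list.
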(event Custom|SelectedNewColor_OnServer
  (params (Remove :type Material%20Interface%20Object%20Reference) (Add :type Material%20Interface%20Object%20Reference))
  (bind _blockcolor (Variables|Default|GetBlockColor))
  (Utilities|Array|RemoveItem _blockcolor Remove)
  (Utilities|Array|Add _blockcolor Add)
  (bind _asbp_lobby_mode (Utilities|Casting|CastToBP_LobbyMode (Game|GetGameMode)))
  (for _array_element (Variables|/Game/TDS/Blueprint/Core/Game/Lobby/BP_LobbyMode.BP_LobbyMode_C|GetPlayerController _asbp_lobby_mode)
    (bind _asbp_lobby_player_controller (Utilities|Casting|CastToBP_LobbyPlayerController _array_element))
    (Default|UpdateColorsLobbyWidgetonClient _asbp_lobby_player_controller (Variables|Default|GetBlockColor))))

(event Custom|AddOrRemoveColorToBlock
  (params (Color :type Material%20Interface%20Object%20Reference) (IsRemove :type Boolean))
  (bind _blockcolor (Variables|Default|GetBlockColor))
  (if IsRemove
    (Utilities|Array|RemoveItem _blockcolor Color)
    (else
      (Utilities|Array|Add _blockcolor Color)))
  (bind _asbp_lobby_mode (Utilities|Casting|CastToBP_LobbyMode (Game|GetGameMode)))
  (for _array_element (Variables|/Game/TDS/Blueprint/Core/Game/Lobby/BP_LobbyMode.BP_LobbyMode_C|GetPlayerController _asbp_lobby_mode)
    (bind _asbp_lobby_player_controller (Utilities|Casting|CastToBP_LobbyPlayerController _array_element))
    (Default|UpdateColorsLobbyWidgetonClient _asbp_lobby_player_controller (Variables|Default|GetBlockColor))))

(event Custom|SelectedNewHat_OnServer
  (params (Remove :type Static%20Mesh%20Object%20Reference) (Add :type Static%20Mesh%20Object%20Reference))
  (bind _blockhatmesh (Variables|Default|GetBlockHatMesh))
  (Utilities|Array|RemoveItem _blockhatmesh Remove)
  (Utilities|Array|Add _blockhatmesh Add)
  (bind _asbp_lobby_mode (Utilities|Casting|CastToBP_LobbyMode (Game|GetGameMode)))
  (for _array_element (Variables|/Game/TDS/Blueprint/Core/Game/Lobby/BP_LobbyMode.BP_LobbyMode_C|GetPlayerController _asbp_lobby_mode)
    (bind _asbp_lobby_player_controller (Utilities|Casting|CastToBP_LobbyPlayerController _array_element))
    (Default|UpdateHatMeshsLobbyWidgetonClient _asbp_lobby_player_controller (Variables|Default|GetBlockHatMesh))))

(event Custom|AddOrRemoveHatToBlock
  (params (HatMesh :type Static%20Mesh%20Object%20Reference) (IsRemove :type Boolean))
  (bind _blockhatmesh (Variables|Default|GetBlockHatMesh))
  (if IsRemove
    (Utilities|Array|RemoveItem _blockhatmesh HatMesh)
    (else
      (Utilities|Array|Add _blockhatmesh HatMesh)))
  (bind _asbp_lobby_mode (Utilities|Casting|CastToBP_LobbyMode (Game|GetGameMode)))
  (for _array_element (Variables|/Game/TDS/Blueprint/Core/Game/Lobby/BP_LobbyMode.BP_LobbyMode_C|GetPlayerController _asbp_lobby_mode)
    (bind _asbp_lobby_player_controller (Utilities|Casting|CastToBP_LobbyPlayerController _array_element))
    (Default|UpdateHatMeshsLobbyWidgetonClient _asbp_lobby_player_controller (Variables|Default|GetBlockHatMesh))))

(fn ConstructionScript)

(fn GetAviableColor
  (for _array_element (Variables|Default|GetAllColor)
    (LocalVariables|SetCanTake true)
    (bind _array_element_2 (Utilities|Array|ForEachLoopwithBreak (Variables|Default|GetBlockColor) :!label _label)
      (:LoopBody
        (if (== _array_element_2 _array_element)
          (LocalVariables|SetCanTake false)
          (goto _label Break)))
      (:Completed
        (if (LocalVariables|GetCanTake)
          (Utilities|Array|Add (LocalVariables|GetAviableColor) _array_element)))))
  (return (LocalVariables|GetAviableColor)))

(fn GetBlockColor
  (return (Variables|Default|GetBlockColor)))

(fn GetBlockHatMesh
  (return (Variables|Default|GetBlockHatMesh)))