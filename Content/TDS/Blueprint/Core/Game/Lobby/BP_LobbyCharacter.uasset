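; Lobby display character that plays idle and ready animations and shows a customizable body material and hat.
; Server events relay color, hat and idle changes to multicasts, which also store the chosen color and hat for remote copies to apply on BeginPlay.
; The authority starts a timer-driven idle loop, with each multicast execution picking its own random montage.
; The ready montage feeds back into that idle loop on completion.
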(event Custom|ChangeColor_OnServer
  (params (TrueColor :type Material%20Interface%20Object%20Reference))
  (CallFunction|ChangeColorMulticast TrueColor))

(event Custom|ChangeColor_Multicast
  (params (NewColor :type Material%20Interface%20Object%20Reference))
  (Rendering|Material|SetMaterial (Variables|Default|GetSkeletalMesh) 0 NewColor)
  (Variables|Default|SetTrueColor NewColor))

(event Custom|MeReady_Multicast
  (Animation|Montage|PlayMontage (Variables|Default|GetSkeletalMesh) "/Game/TDS/Blueprint/Core/Game/Lobby/Animation/AM_ReadyLobby.AM_ReadyLobby"
    (:OnCompleted
      (CallFunction|WaitAnimMulticast))))

(event Custom|WaitAnimation_OnServer
  (CallFunction|WaitAnimMulticast))

(event Custom|ChangeHatMesh_OnServer
  (params (TrueHatMesh :type Static%20Mesh%20Object%20Reference))
  (CallFunction|ChangeHatMeshMulticast TrueHatMesh))

(event Custom|ChangeHatMesh_Multicast
  (params (TrueHatMesh :type Static%20Mesh%20Object%20Reference))
  (Components|StaticMesh|SetStaticMesh (Variables|Default|GetHat) TrueHatMesh)
  (Variables|Default|SetTrueHatMesh TrueHatMesh))

(event Custom|WaitAnim_Multicast
  (bind _waitanim (Variables|Default|GetWaitAnim))
  (Animation|Montage|PlayMontage (Variables|Default|GetSkeletalMesh) (Utilities|Array|Get(acopy) _waitanim (Math|Random|RandomInteger (Utilities|Array|Length _waitanim)))
    (:OnCompleted
      (Utilities|Time|SetTimerbyEvent (delegate Custom|WaitAnimation_OnServer) 2.0))))

(event EventBeginPlay
  (Networking|SwitchHasAuthority
    (:Authority
      (Utilities|Time|SetTimerbyEvent (delegate Custom|WaitAnimation_OnServer) 2.0))
    (:Remote
      (Rendering|Material|SetMaterial (Variables|Default|GetSkeletalMesh) 0 (Variables|Default|GetTrueColor))
      (Components|StaticMesh|SetStaticMesh (Variables|Default|GetHat) (Variables|Default|GetTrueHatMesh)))))

(fn ConstructionScript)