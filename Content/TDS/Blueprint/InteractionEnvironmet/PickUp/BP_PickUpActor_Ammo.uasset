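; Ammo pickup actor that refills a weapon type's ammo in the overlapping character's inventory.
; On BeginPlay, InitActor picks the mesh and Niagara effect from the weapon ammo type, destroying either component when no asset is mapped, as for Pistol.
; The parent's OverlapCharacter event is extended to check whether the inventory can take that ammo, add the count and signal pickup success only then.
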(event EventBeginPlay
  (|CallParentFunction)
  (CallFunction|InitActor))

(event Collision|EventActorBeginOverlap
  (params (OtherActor :type Actor%20Object%20Reference))
  (|CallParentFunction OtherActor) ; This node is disabled and will not be called.\nDrag off pins to build functionality.
)

(event EventTick
  (params (DeltaSeconds :type Float%20%28single-precision%29))
  (|CallParentFunction DeltaSeconds) ; This node is disabled and will not be called.\nDrag off pins to build functionality.
)

(event EventOverlapCharacter
  (params (ToInventory :type TDS%20Inventory%20Component%20Object%20Reference))
  (bind _weapontypeammo (Variables|Default|GetWeaponTypeAmmo))
  (|CallParentFunction ToInventory)
  (bind _returnvalue (Class|TDSInventoryComponent|CheckCanTakeAmmo ToInventory _weapontypeammo))
  (if _returnvalue
    (Class|TDSInventoryComponent|AmmoSlotChangeValue ToInventory _weapontypeammo (Variables|Default|GetCout))
    (CallFunction|PickUpSuccess)))

(fn ConstructionScript
  (|CallParentFunction))

(fn InitActor
  (bind _weapontypeammo (Variables|Default|GetWeaponTypeAmmo))
  (bind _staticmesh (Variables|Default|GetStaticMesh))
  (bind _niagara (Variables|Default|GetNiagara))
  (bind _returnvalue (Utilities|Select :Index _weapontypeammo :RifleMKType "/Game/TDS/Items/GameActor/Weapon/Weapons_Model/Meshes/AR4/SM_AR4_Mag_Empty.SM_AR4_Mag_Empty" :RifleAKType "/Game/TDS/Items/GameActor/Weapon/Weapons_Model/Meshes/Ka47/SM_KA47_Mag_Empty.SM_KA47_Mag_Empty" :PistolType 0 :ShotGunType "/Game/TDS/Items/GameActor/Weapon/Weapons_Model/Meshes/Low_Poligon/SM_Weapon_01_4.SM_Weapon_01_4" :SniperRifle "/Game/TDS/Items/GameActor/Weapon/Weapons_Model/Meshes/KA_Val/SM_KA_Val_MAG_Loaded_Y.SM_KA_Val_MAG_Loaded_Y" :GrenadeLauncher "/Game/TDS/Items/GameActor/Weapon/Weapons_Model/Meshes/Low_Poligon/SM_Weapon_01_4.SM_Weapon_01_4" :RocketLauncher "/Game/TDS/Items/GameActor/Weapon/Weapons_Model/Meshes/Low_Poligon/SM_Weapon_01_4.SM_Weapon_01_4"))
  (bind _returnvalue_2 (Utilities|Select :Index _weapontypeammo :RifleMKType "/Game/TDS/Items/GameActor/Weapon/Weapon_FX/NS_Rifle.NS_Rifle" :RifleAKType "/Game/TDS/Items/GameActor/Weapon/Weapon_FX/NS_Rifle.NS_Rifle" :PistolType 0 :ShotGunType "/Game/TDS/Items/GameActor/Weapon/Weapon_FX/NS_Shotgun.NS_Shotgun" :SniperRifle "/Game/TDS/Items/GameActor/Weapon/Weapon_FX/NS_SniperRifle.NS_SniperRifle" :GrenadeLauncher "/Game/TDS/Items/GameActor/Weapon/Weapon_FX/NS_GranadeLauncher.NS_GranadeLauncher" :RocketLauncher "/Game/TDS/Items/GameActor/Weapon/Weapon_FX/NS_RocketLauncher.NS_RocketLauncher"))
  (Utilities|FlowControl|Sequence
    (:then_0
      (Utilities|IsValid _returnvalue
        (:Is%20Valid
          (Components|StaticMesh|SetStaticMesh _staticmesh _returnvalue)
          (Transformation|SetRelativeLocation _staticmesh "0, 0, 0" false false)
          (Transformation|SetRelativeScale3D _staticmesh "2.000000,2.000000,2.000000")
          (Transformation|SetRelativeRotation _staticmesh "0.000000,0.000000,-80.000000" false false))
        (:Is%20Not%20Valid
          (Components|DestroyComponent _staticmesh))))
    (:then_1
      (Utilities|IsValid _returnvalue_2
        (:Is%20Valid
          (Class|NiagaraComponent|SetAsset _niagara _returnvalue_2 true)
          (Transformation|SetRelativeScale3D _niagara "1.000000,1.000000,1.000000"))
        (:Is%20Not%20Valid
          (Components|DestroyComponent _niagara))))))