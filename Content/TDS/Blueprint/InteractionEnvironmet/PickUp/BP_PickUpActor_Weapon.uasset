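; Weapon pickup actor that shows a dropped weapon in the world.
; On BeginPlay it looks up drop info by ItemName in BP_GameInstance, then InitActor applies a static or skeletal mesh and optional Niagara effect, destroying unused components.
; Leaving the sphere notifies BP_TopDownCharacter.
; Overlap handling only calls the parent; the graph's inventory-add and weapon-switch logic is disconnected.
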(event OnComponentEndOverlap(Sphere)
  (params (OverlappedComponent :type Primitive%20Component%20Object%20Reference) (OtherActor :type Actor%20Object%20Reference) (OtherComp :type Primitive%20Component%20Object%20Reference) (OtherBodyIndex :type Integer))
  (bind _asbp_top_down_character (Utilities|Casting|CastToBP_TopDownCharacter OtherActor))
  (Default|EndOverlapwithPickUpWeapon _asbp_top_down_character))

(event EventBeginPlay
  (bind _itemname (Variables|Default|GetItemName))
  (|CallParentFunction)
  (if (!= _itemname "")
    (bind _asbp_game_instance (Utilities|Casting|CastToBP_GameInstance (Game|GetGameInstance)))
    (bind (_outinfo _returnvalue) (Class|TDSGameInstance|GetDropItemInfobyName _asbp_game_instance _itemname))
    (if _returnvalue
      (Variables|Default|SetWeaponInfo _outinfo)))
  (CallFunction|InitActor (Variables|Default|GetWeaponInfo)))

(event Collision|EventActorBeginOverlap
  (params (OtherActor :type Actor%20Object%20Reference))
  (|CallParentFunction OtherActor) ; This node is disabled and will not be called.\nDrag off pins to build functionality.
)

(event EventTick
  (params (DeltaSeconds :type Float%20%28single-precision%29))
  (|CallParentFunction DeltaSeconds) ; This node is disabled and will not be called.\nDrag off pins to build functionality.
)

(event EventOverlapCharacter
  (params (ToInventory :type TDS%20Inventory%20Component%20Object%20Reference))
  (|CallParentFunction ToInventory))

(fn ConstructionScript
  (|CallParentFunction))

(fn InitActor
  (params (InfoActor :type Drop%20Item%20Structure))
  (bind (_weaponstaticmesh _weaponskeletalmesh _niagaraitem _offset _weaponinfo) (Utilities|Struct|BreakDropItem InfoActor))
  (bind _staticmesh (Variables|Default|GetStaticMesh))
  (bind _skeletalmesh (Variables|Default|GetSkeletalMesh))
  (bind _niagara (Variables|Default|GetNiagara))
  (Utilities|FlowControl|Sequence
    (:then_0
      (Utilities|IsValid _weaponstaticmesh
        (:Is%20Valid
          (Components|DestroyComponent (Variables|Default|GetSkeletalMesh))
          (Components|StaticMesh|SetStaticMesh _staticmesh _weaponstaticmesh)
          (Transformation|SetRelativeLocation _staticmesh (.location _offset) false false)
          (Transformation|SetRelativeRotation _staticmesh (.rotation _offset) false false))
        (:Is%20Not%20Valid
          (Utilities|IsValid _weaponskeletalmesh
            (:Is%20Valid
              (Components|DestroyComponent (Variables|Default|GetStaticMesh))
              (Components|SkeletalMesh|SetSkeletalMeshAsset _skeletalmesh _weaponskeletalmesh)
              (Transformation|SetRelativeLocation _skeletalmesh (.location _offset) false false))
            (:Is%20Not%20Valid
              (Development|PrintString "Error Drop Item || NO MESH"))))))
    (:then_1
      (Utilities|IsValid _niagaraitem
        (:Is%20Valid
          (Class|NiagaraComponent|SetAsset _niagara _niagaraitem true)
          (Transformation|SetRelativeScale3D _niagara (.scale _offset)))
        (:Is%20Not%20Valid
          (Components|DestroyComponent _niagara))))
    (:then_2
      (Variables|Default|SetItemName (.NameItem (Utilities|Struct|BreakWeaponSlot _weaponinfo))))))