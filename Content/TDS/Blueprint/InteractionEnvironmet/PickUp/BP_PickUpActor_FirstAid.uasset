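; First-aid pickup actor that restores health to the top-down character who picks it up.
; It overrides the parent pickup's OverlapCharacter event and casts the inventory's owner to BP_TopDownCharacter.
; If that character's current health is below a hard-coded 100, it applies its Value through the health component's server call and completes the pickup.
; At or above that threshold, the pickup is not completed.
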(event EventBeginPlay
  (|CallParentFunction) ; This node is disabled and will not be called.\nDrag off pins to build functionality.
)

(event Collision|EventActorBeginOverlap
  (params (OtherActor :type Actor%20Object%20Reference))
  (|CallParentFunction OtherActor) ; This node is disabled and will not be called.\nDrag off pins to build functionality.
)

(event EventTick
  (params (DeltaSeconds :type Float%20%28single-precision%29))
  (|CallParentFunction DeltaSeconds) ; This node is disabled and will not be called.\nDrag off pins to build functionality.
)

(event EventOverlapCharacter
  (params (ToInventory :type TDS%20Inventory%20Component%20Object%20Reference))
  (|CallParentFunction ToInventory)
  (bind _asbp_top_down_character (Utilities|Casting|CastToBP_TopDownCharacter (Components|GetOwner ToInventory)))
  (bind _returnvalue (Class|TDSHealthComponent|GetCurrentHealth (Variables|/Script/TDS.TDSCharacter|GetCharHealthComponent _asbp_top_down_character)))
  (if (< _returnvalue 1e+02)
    (Class|TDSHealthComponent|ChangeHealthValueonServer (Variables|/Script/TDS.TDSCharacter|GetCharHealthComponent _asbp_top_down_character) (Variables|Default|GetValue))
    (CallFunction|PickUpSuccess)))

(fn ConstructionScript
  (|CallParentFunction))