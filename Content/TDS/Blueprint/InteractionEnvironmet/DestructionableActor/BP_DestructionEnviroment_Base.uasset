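; Base destructible environment actor for TDS that takes damage, shows floating damage numbers and can drop pickups.
; Damage feeds the TDSHealth component, while radial projectile hits also apply the projectile's effect based on the mesh's physical surface.
; On death it optionally spawns a first-aid or random weapon pickup using a downward trace, then destroys itself with explosion and collapse sound.
; Tick prints active effect names for debugging.
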(event OnHealthChange(TDSHealth)
  (params (Health :type Float%20%28single-precision%29) (Damage :type Float%20%28single-precision%29))
  (bind _returnvalue (Game|SpawnActorfromClass "/Game/TDS/Blueprint/InteractionEnvironmet/DisplayDamage/BP_DisplayDamage.BP_DisplayDamage_C" (Math|Transform|MakeTransform (+ (Transformation|GetActorLocation) (+ (Variables|Default|GetLocalPointSpawnHealthNumber) (Math|Vector|MakeVector (Math|Random|RandomFloatinRange -2e+01 2e+01) (Math|Random|RandomFloatinRange -2e+01 2e+01) 0.0)))) "Undefined" "MultiplyWithRoot" 0 0))
  (Default|InitActor _returnvalue Health Damage))

(event OnDead(TDSHealth)
  (Utilities|FlowControl|Delay 0.0001)
  (if (Variables|Default|GetIsDrop)
    (CallFunction|Drop))
  (CallFunction|DestroyActor))

(event EventBeginPlay)

(event Collision|EventActorBeginOverlap
  (params (OtherActor :type Actor%20Object%20Reference)))

(event EventTick
  (params (DeltaSeconds :type Float%20%28single-precision%29))
  (for _array_element (Variables|Default|GetEffects)
    (Development|PrintString (Utilities|GetDisplayName _array_element) true true "(R=0.000000,G=0.660000,B=1.000000,A=1.000000)" 0.0)))

(event Game|Damage|EventAnyDamage
  (params (Damage :type Float%20%28single-precision%29) (DamageType :type Damage%20Type%20Object%20Reference) (InstigatedBy :type Controller%20Object%20Reference) (DamageCauser :type Actor%20Object%20Reference))
  (Class|TDSHealthComponent|ChangeHealthValueonServer (Variables|Default|GetTDSHealth) (* Damage -1.0)))

(event Game|Damage|EventRadialDamage
  (params (DamageReceived :type Float%20%28single-precision%29) (DamageType :type Damage%20Type%20Object%20Reference) (Origin :type Vector :default "0, 0, 0") (HitInfo :type Hit%20Result%20Structure%20%28by%20ref%29) (InstigatedBy :type Controller%20Object%20Reference) (DamageCauser :type Actor%20Object%20Reference))
  (bind _asprojectile_default (Utilities|Casting|CastToProjectileDefault DamageCauser))
  (Class|Types|AddEffectbySurfaceType self "None" (.Effect (Utilities|Struct|BreakProjectileInfo (Variables|/Script/TDS.ProjectileDefault|GetProjectileSetting _asprojectile_default))) (Variables|/Script/PhysicsCore.PhysicalMaterial|GetSurfaceType (Class|MaterialInterface|GetPhysicalMaterial (Rendering|Material|GetMaterial (Variables|Default|GetStaticMesh) 0)))))

(fn ConstructionScript)

(fn DestroyActor
  (bind _returnvalue (Transformation|GetActorLocation))
  (Actor|DestroyActor)
  (Audio|SpawnSoundatLocation "/Game/StarterContent/Audio/Collapse01.Collapse01" _returnvalue "0, 0, 0" 1.0 1.0 0.0 0 0)
  (Effects|SpawnEmitteratLocation "/Game/StarterContent/Particles/P_Explosion.P_Explosion" _returnvalue))

(fn Drop
  (bind _returnvalue (Transformation|GetActorLocation))
  (bind _returnvalue_2 (Transformation|GetActorLocation))
  (if (Variables|Default|GetIsHealth)
    (bind _outhit (Collision|LineTraceByChannel _returnvalue_2 (+ _returnvalue_2 "0.000000,0.000000,-200.000000") "TraceTypeQuery1" false 0 "None"))
    (Game|SpawnActorfromClass "/Game/TDS/Blueprint/InteractionEnvironmet/PickUp/BP_PickUpActor_FirstAid.BP_PickUpActor_FirstAid_C" (Math|Transform|MakeTransform (.Location (Collision|BreakHitResult _outhit))) "AlwaysSpawn" "MultiplyWithRoot" 0 0)
    (else
      (bind _outhit_2 (Collision|LineTraceByChannel _returnvalue (+ _returnvalue "0.000000,0.000000,-200.000000") "TraceTypeQuery1" false 0 "None"))
      (Game|SpawnActorfromClass :Class "/Game/TDS/Blueprint/InteractionEnvironmet/PickUp/BP_PickUpActor_Weapon.BP_PickUpActor_Weapon_C" :SpawnTransform (Math|Transform|MakeTransform (Math|Vector|MakeVector (.x (.Location (Collision|BreakHitResult _outhit_2))) (.y (.Location (Collision|BreakHitResult _outhit_2))) 2e+01)) :CollisionHandlingOverride "AlwaysSpawn" :TransformScaleMethod "MultiplyWithRoot" :ItemName (Utilities|Array|Get(acopy) (Variables|Default|GetDropWeapon) (Math|Random|RandomIntegerinRange 0 4)) :Instigator 0))))